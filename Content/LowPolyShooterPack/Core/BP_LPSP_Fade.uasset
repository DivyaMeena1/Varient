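; BP_LPSP_Fade plays a fade level sequence when play begins and keeps the player from acting during it.
; On BeginPlay it disables the first player character's input, then creates and plays a sequence player for FadeSequence.
; Input returns after a configurable delay, PlayerInputEnableDelay, through OnSequenceStop, which is timer-driven rather than bound to the sequence's actual end.
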(event `self.ReceiveBeginPlay`
  ;[0.7812 1 0] Begin Play
  (`parent.ReceiveBeginPlay`)
  (`self.DisableInput` (`GameplayStatics.GetPlayerCharacter` 0) (`GameplayStatics.GetPlayerController` 0))
  (bind (_outactor _returnvalue) (`LevelSequencePlayer.CreateLevelSequencePlayer` (`self.Fade Sequence`)))
  (`MovieSceneSequencePlayer.Play` _returnvalue)
  (`KismetSystemLibrary.Delay` (`self.Player Input Enable Delay`))
  (`self.On Sequence Stop`))

(event `On Sequence Stop`
  ;[1 1 1] On Sequence Stop
  (`self.EnableInput` (`GameplayStatics.GetPlayerCharacter` 0) (`GameplayStatics.GetPlayerController` 0)))

(fn `UserConstructionScript`)