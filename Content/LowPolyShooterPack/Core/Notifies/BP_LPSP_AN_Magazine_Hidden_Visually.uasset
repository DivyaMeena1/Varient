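; Animation notify that shows or hides the magazine mesh of the player's equipped weapon during an animation.
; On trigger it gets player character 0, queries its current weapon actor through an interface message, and caches it.
; If that weapon is valid, it sends the weapon a set-magazine-hidden-visually message with the notify's Hidden flag.
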(fn `GetNotifyName`
  (returns (ReturnValue :type String))
  (return "Set Magazine Hidden Visually"))

(fn `Received_Notify`
  (params (MeshComp :type "SkeletalMeshComponent Object Reference") (Animation :type "AnimSequenceBase Object Reference"))
  (returns (ReturnValue :type Boolean))
  (locals (`Actor Weapon` :type "Actor Object Reference"))
  (`|ExecutionSequence`
    (:`then_0`
      (`/Engine/EditorBlueprintResources/StandardMacros.IsValid` (`GameplayStatics.GetPlayerCharacter` 0)
        (:`Is Valid`
          (bind _returnvalue (message `/Game/LowPolyShooterPack/Core/Characters/BPI_LPSP_CH.Get Actor Weapon` (`GameplayStatics.GetPlayerCharacter` 0)))
          (bind _output_get (set `local.Actor Weapon` _returnvalue))
          (`/Engine/EditorBlueprintResources/StandardMacros.IsValid` _output_get
            (:`Is Valid`
              (message `/Game/LowPolyShooterPack/Core/Weapons/BPI_LPSP_WEP.On Set Hidden Magazine Visually` (`local.Actor Weapon`) (`self.Hidden`)))))))
    (:`then_1`
      (return true))))