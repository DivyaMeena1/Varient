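; Animation notify that lands the player's melee hit at a chosen moment in an animation.
; Sphere-traces forward from the player camera on the Visibility channel, ignoring the player, then spawns surface-specific details at the hit.
; Damageable actors receive zero point damage, because the current systems treat any damage as maximum.
; Physics-simulating components are pushed with an impulse along the trace direction.
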(fn `GetNotifyName`
  (returns (ReturnValue :type String))
  (return "Melee"))

(fn `Received_Notify`
  (params (MeshComp :type "SkeletalMeshComponent Object Reference") (Animation :type "AnimSequenceBase Object Reference"))
  (returns (ReturnValue :type Boolean))
  (locals (Hit :type "HitResult Structure"))
  (bind _returnvalue (`GameplayStatics.GetPlayerCameraManager` 0))
  (bind (_bblockinghit _binitialoverlap _time _distance _location _impactpoint _normal _impactnormal _physmat _hitactor _hitcomponent _hitbonename _hititem _faceindex _tracestart _traceend) (`GameplayStatics.BreakHitResult` (`local.Hit`)))
  (bind (_bblockinghit_2 _binitialoverlap_2 _time_2 _distance_2 _location_2 _impactpoint_2 _normal_2 _impactnormal_2 _physmat_2 _hitactor_2 _hitcomponent_2 _hitbonename_2) (`GameplayStatics.BreakHitResult` (`local.Hit`)))
  (bind (_bblockinghit_3 _binitialoverlap_3 _time_3 _distance_3 _location_3 _impactpoint_3 _normal_3 _impactnormal_3 _physmat_3 _hitactor_3 _hitcomponent_3 _hitbonename_3) (`GameplayStatics.BreakHitResult` (`local.Hit`)))
  (`|ExecutionSequence`
    (:`then_0`
      ;[1 0.2344 0 1 12] Simple linetrace to the front of the camera.
      (bind (_outhit _returnvalue_2) (`KismetSystemLibrary.SphereTraceSingle` (`PlayerCameraManager.GetCameraLocation` (`GameplayStatics.GetPlayerCameraManager` 0)) (+ (`PlayerCameraManager.GetCameraLocation` _returnvalue) (* (`Actor.GetActorForwardVector` _returnvalue) (`self.Range`))) (`self.Trace Radius`) "TraceTypeQuery1" false (`|MakeArray` (`GameplayStatics.GetPlayerCharacter` 0) :!type "Actor Object Reference")))
      (set `local.Hit` _outhit)
      (if _returnvalue_2
        ;[0 1 0.25 1 12] Spawn all the cool effects.
        (`/Game/LowPolyShooterPack/Core/Surfaces/BPFL_LPSP_Surfaces.Spawn Surface Details` _outhit (`self.Surfaces Handle`))
        (`|ExecutionSequence`
          (:`then_0`
            ;[0 0.03906 1 1 12] We don't apply any damage, since our current systems consider any damage max damage.
            (bind _asbp_lpsp_damageable (cast `/Game/LowPolyShooterPack/Core/Damageables/BP_LPSP_Damageable` (`.HitActor` (`GameplayStatics.BreakHitResult` _outhit))))
            (`LPSPDamageable.PointDamage` _asbp_lpsp_damageable 0.0 (`GameplayStatics.GetPlayerCharacter` 0)))
          (:`then_1`
            ;[0.6875 1 0 1 12] Add some nice impulses!
            (if (`SceneComponent.IsSimulatingPhysics` _hitcomponent_2 _hitbonename_2)
              (`PrimitiveComponent.AddImpulseAtLocation` _hitcomponent_3 (* (`KismetMathLibrary.Normal` (- _traceend _tracestart)) (`self.Impulse`)) _impactpoint_3 _hitbonename_3))))))
    (:`then_1`
      (return true))))