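; SaveGame object for the Low Poly Shooter Pack that stores the player's video and audio settings.
; Getter and setter pairs expose display, graphics quality and volume values, covering master, music, SFX and ambience.
; Setters for vertical sync, quality levels and resolution scale clamp their input, while screen resolution, fullscreen mode and volumes are stored unclamped.
; It only holds values and contains no logic to apply or save them.
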(fn `Get Index Anti Aliasing`
  (returns (ReturnValue :type Integer))
  (return (`self.Index Anit Aliasing`)))

(fn `Get Index Fullscreen Mode`
  (returns (ReturnValue :type Integer))
  (return (`self.Index Fullscreen Mode`)))

(fn `Get Index Post Processing Quality`
  (returns (ReturnValue :type Integer))
  (return (`self.Index Post Processing Quality`)))

(fn `Get Index Screen Resolution`
  (returns (ReturnValue :type Integer))
  (return (`self.Index Screen Resolution`)))

(fn `Get Index Shadow Quality`
  (returns (ReturnValue :type Integer))
  (return (`self.Index Shadow Quality`)))

(fn `Get Index Texture Quality`
  (returns (ReturnValue :type Integer))
  (return (`self.Index Texture Quality`)))

(fn `Get Index Vertical Sync`
  (returns (ReturnValue :type Integer))
  (return (`self.Index Vertical Sync`)))

(fn `Get Value Resolution Scale`
  (returns (ReturnValue :type "Float (double-precision)"))
  (return (`self.Value Resolution Scale`)))

(fn `Get Value Volume Ambience`
  (returns (ReturnValue :type "Float (double-precision)"))
  (return (`self.Value Volume Ambience`)))

(fn `Get Value Volume Master`
  (returns (ReturnValue :type "Float (double-precision)"))
  (return (`self.Value Volume Master`)))

(fn `Get Value Volume Music`
  (returns (ReturnValue :type "Float (double-precision)"))
  (return (`self.Value Volume Music`)))

(fn `Get Value Volume SFX`
  (returns (ReturnValue :type "Float (double-precision)"))
  (return (`self.Value Volume SFX`)))

(fn `Set Index Fullscreen Mode`
  (params (Value :type Integer))
  (set `self.Index Fullscreen Mode` Value)
  (return))

(fn `Set Index Screen Resolution`
  (params (Value :type Integer))
  (set `self.Index Screen Resolution` Value)
  (return))

(fn `Set Value Anti Aliasing`
  (params (Value :type Integer))
  (set `self.Index Anit Aliasing` (`KismetMathLibrary.Clamp` Value 0 3))
  (return))

(fn `Set Value Post Processing Quality`
  (params (Value :type Integer))
  (set `self.Index Post Processing Quality` (`KismetMathLibrary.Clamp` Value 0 3))
  (return))

(fn `Set Value Resolution Scale`
  (params (Value :type "Float (double-precision)"))
  (set `self.Value Resolution Scale` (`KismetMathLibrary.FClamp` Value))
  (return))

(fn `Set Value Shadow Quality`
  (params (Value :type Integer))
  (set `self.Index Shadow Quality` (`KismetMathLibrary.Clamp` Value 0 3))
  (return))

(fn `Set Value Texture Quality`
  (params (Value :type Integer))
  (set `self.Index Texture Quality` (`KismetMathLibrary.Clamp` Value 0 3))
  (return))

(fn `Set Value Vertical Sync`
  (params (Value :type Integer))
  (set `self.Index Vertical Sync` (`KismetMathLibrary.Clamp` Value 0 1))
  (return))

(fn `Set Value Volume Ambience`
  (params (Value :type "Float (double-precision)"))
  (set `self.Value Volume Ambience` Value)
  (return))

(fn `Set Value Volume Master`
  (params (Value :type "Float (double-precision)"))
  (set `self.Value Volume Master` Value)
  (return))

(fn `Set Value Volume Music`
  (params (Value :type "Float (double-precision)"))
  (set `self.Value Volume Music` Value)
  (return))

(fn `Set Value Volume SFX`
  (params (Value :type "Float (double-precision)"))
  (set `self.Value Volume SFX` Value)
  (return))