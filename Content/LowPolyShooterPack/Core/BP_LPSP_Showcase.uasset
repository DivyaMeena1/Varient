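; BP_LPSP_Showcase is a Low Poly Shooter Pack actor that displays a weapon through a child actor component.
; The construction script previews the first class in its Weapons array.
; On BeginPlay it swaps in a random class from that array, then sends the spawned weapon a physical-settings message pointing to the Static row of DT_LPSP_WEP_Physical.
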(event `self.ReceiveBeginPlay`
  ;[1 0.7031 0] Begin Play
  (`parent.ReceiveBeginPlay`)
  (`ChildActorComponent.SetChildActorClass` (`self.Weapon`) (`KismetArrayLibrary.Array_Random` (`self.Weapons`))) ; Update Weapon Class
  (message `/Game/LowPolyShooterPack/Core/Weapons/BPI_LPSP_WEP.On Change Settings Physical` (`ChildActorComponent.ChildActor` (`self.Weapon`)) (make `DataTableRowHandle` "/Game/LowPolyShooterPack/Data/Weapons/DT_LPSP_WEP_Physical.DT_LPSP_WEP_Physical" "Static")))

(fn `UserConstructionScript`
  (`parent.UserConstructionScript`)
  (`ChildActorComponent.SetChildActorClass` (`self.Weapon`) (`|GetArrayItem` (`self.Weapons`))))