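; BP_LPSP_DMG_Gas is a damageable gas prop that turns into a flaming, self-propelled object when shot.
; The first point-damage hit toggles main and sideways thrusters and activates flame audio and particles; the next hit kills it.
; On BeginPlay, both thrusters get random strengths scaled by mesh mass.
; The construction script randomizes the flame particle size.
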(event `self.On Damaged Point`
  ;[0 0.3203 1 1 12] Damage (Point)
  (if (`self.bHit`)
    (`self.Kill`)
    (else
      (set `self.bHit` true)
      (`parent.On Damaged Point`)
      (`ActorComponent.ToggleActive` (`self.Thruster`))
      (`ActorComponent.ToggleActive` (`self.Thruster Sideways`))
      (`ActorComponent.Activate` (`self.Flames Audio`) true)
      (`ActorComponent.Activate` (`self.Flames Particles`) true))))

(event `self.ReceiveBeginPlay`
  (bind (_thruster_strength_x _thruster_strength_y) (`KismetMathLibrary.BreakVector2D` (`self.Thruster Strength`)))
  (bind (_thruster_strength__sideways__x _thruster_strength__sideways__y) (`KismetMathLibrary.BreakVector2D` (`self.Thruster Strength (Sideways)`)))
  ;[1 0 0.07031 1 12] Begin Play
  (`parent.ReceiveBeginPlay`)
  (set `PhysicsThrusterComponent.ThrustStrength` (* (`KismetMathLibrary.RandomFloatInRange` _thruster_strength_x _thruster_strength_y) (`PrimitiveComponent.GetMass` (`self.Mesh`))) (`self.Thruster`))
  (set `PhysicsThrusterComponent.ThrustStrength` (* (`KismetMathLibrary.RandomFloatInRange` _thruster_strength__sideways__x _thruster_strength__sideways__y) (`PrimitiveComponent.GetMass` (`self.Mesh`))) (`self.Thruster Sideways`)))

(fn `UserConstructionScript`
  (bind (_flame_particles__size__x _flame_particles__size__y) (`KismetMathLibrary.BreakVector2D` (`self.Flame Particles (Size)`)))
  (`parent.UserConstructionScript`)
  (`SceneComponent.SetWorldScale3D` (`self.Flames Particles`) (`KismetMathLibrary.Conv_DoubleToVector` (`KismetMathLibrary.RandomFloatInRange` _flame_particles__size__x _flame_particles__size__y))))