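; Damageable shooting target that drops when hit by point damage and raises itself again.
; A Lowered flag ignores repeat hits while collapsed graphs show a hit-text widget and play the lower sound and animation.
; After a random delay within ResetDelay, it clears the flag and plays the reset sound and animation.
; On death, it calls the parent handler and spawns the optional destroyed-version actor at the mesh's target socket.
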(event `self.On Damaged Point`
  (bind (_reset_delay_x _reset_delay_y) (`KismetMathLibrary.BreakVector2D` (`self.Reset Delay`)))
  ;[0.2656 1 0] Point Damage
  (if (not (`self.Lowered`))
    (set `self.Lowered` true)
    (bind _returnvalue (`|CreateWidget` (`self.Hit Text Widget`)))
    (`UserWidget.AddToViewport` _returnvalue 0)
    (`GameplayStatics.PlaySoundAtLocation` (`self.Lower Sound`) (`SceneComponent.K2_GetComponentLocation` (`self.Target Mesh`)) (struct) 1.0 1.0 0.0 null null null)
    (`SkeletalMeshComponent.PlayAnimation` (`self.Target Mesh`) (`self.Lower Sequence`) false)
    (`|ExecutionSequence`
      (:`then_0`
        (`KismetSystemLibrary.Delay` (`KismetMathLibrary.RandomFloatInRange` _reset_delay_x _reset_delay_y))
        (set `self.Lowered` false)
        (`GameplayStatics.PlaySoundAtLocation` (`self.Reset Sound`) (`SceneComponent.K2_GetComponentLocation` (`self.Target Mesh`)) (struct) 1.0 1.0 0.0 "/Game/LowPolyShooterPack/Audio/ATT_Weapons.ATT_Weapons" null null)
        (`SkeletalMeshComponent.PlayAnimation` (`self.Target Mesh`) (`self.Reset Sequence`) false))
      (:`then_1`))))

(event `self.On Has Died`
  ;[1 0.8203 0] Death
  (`parent.On Has Died`)
  (if (`KismetSystemLibrary.IsValidClass` (`self.Destroyed Version Class`))
    (`|SpawnActorFromClass` (`self.Destroyed Version Class`) (`SceneComponent.GetSocketTransform` (`self.Target Mesh`) "SOCKET_Target" "RTS_World") "AlwaysSpawn" "OverrideRootScale" null null) ; Spawn Destroyed
  ))

(fn `UserConstructionScript`
  (`parent.UserConstructionScript`))