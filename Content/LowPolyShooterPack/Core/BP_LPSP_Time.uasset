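; BP_LPSP_Time is a time-control Blueprint in the Low Poly Shooter Pack that lets the player slow down, speed up or pause the game.
; Speed-up and slow-down inputs step a target time scale by a set increment, clamped between zero and normal speed.
; Tick smoothly interpolates global time dilation toward that target.
; The stop input uses a FlipFlop to toggle game pause.
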(event `self.ReceiveBeginPlay`
  ;[0.3125 0 1] Begin Play
  (`parent.ReceiveBeginPlay`)
  (set `self.Time Scale (Current)` (`self.Time Scale Default`)))

(event `self.ReceiveTick`
  (params (DeltaSeconds :type "Float (single-precision)"))
  ;[0.125 0 1] Tick
  (`parent.ReceiveTick` DeltaSeconds)
  (`GameplayStatics.SetGlobalTimeDilation` (`KismetMathLibrary.FInterpTo` (`GameplayStatics.GetGlobalTimeDilation`) (`self.Time Scale (Current)`) DeltaSeconds 20.0)))

(event `InputAction|Time Speed Up`
  (params (Key :type "Key Structure"))
  ;[1 0 0.6562] Increase
  (:`Pressed`
    (`self.Update Time Scale` (+ (`self.Time Scale (Current)`) (`self.Time Scale Increments`)))))

(event `InputAction|Time Slow Down`
  (params (Key :type "Key Structure"))
  ;[0.6641 0 1] Decrease
  (:`Pressed`
    (`self.Update Time Scale` (- (`self.Time Scale (Current)`) (`self.Time Scale Increments`)))))

(event `InputAction|Time Stop` :paused true
  (params (Key :type "Key Structure"))
  ;[1 0 0.6094] Stop
  (:`Pressed`
    (`/Engine/EditorBlueprintResources/StandardMacros.FlipFlop`
      (:`A`
        (`GameplayStatics.SetGamePaused` true))
      (:`B`
        (`GameplayStatics.SetGamePaused` false)))))

(fn `Update Time Scale`
  (params (Value :type "Float (double-precision)"))
  (bind _returnvalue (`KismetMathLibrary.FClamp` Value))
  (`|ExecutionSequence`
    (:`then_0`
      (if (not (== (`self.Time Scale (Current)`) _returnvalue))
        (set `self.Time Scale (Current)` _returnvalue)))
    (:`then_1`
      (return))))

(fn `UserConstructionScript`)