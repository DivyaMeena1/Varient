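; Sci-fi assault rifle weapon Blueprint in the Low Poly Shooter Pack that adds a jetpack effect when the character jumps.
; On the jump event it spawns jetpack particles on the player's capsule and traces downward to spawn surface-specific details.
; It also uses an explosion component to shake, apply damage at once and apply an impulse after a short delay.
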(event `/Game/LowPolyShooterPack/Core/Weapons/BPI_LPSP_WEP.On Character Jumped`
  ;[0 0.9766 1] Event Character Jumped
  (`GameplayStatics.SpawnEmitterAttached` (`self.Jetpack Particles`) (`Character.CapsuleComponent` (`GameplayStatics.GetPlayerCharacter` 0)) "None" (0.0 0.0 60.0) (struct :`Yaw` -90.0))
  (bind _outhit (`KismetSystemLibrary.LineTraceSingle` (`self.K2_GetActorLocation` (`GameplayStatics.GetPlayerCharacter` 0)) (+ (`self.K2_GetActorLocation` (`GameplayStatics.GetPlayerCharacter` 0)) (* (* (`KismetMathLibrary.NegateVector` (`KismetMathLibrary.GetUpVector` (`self.K2_GetActorRotation` (`GameplayStatics.GetPlayerCharacter` 0)))) (`CapsuleComponent.CapsuleHalfHeight` (`Character.CapsuleComponent` (`GameplayStatics.GetPlayerCharacter` 0)))) 1.2)) "TraceTypeQuery1" false (`|MakeArray` self :!type "Actor Object Reference")))
  (`/Game/LowPolyShooterPack/Core/Surfaces/BPFL_LPSP_Surfaces.Spawn Surface Details` _outhit (`self.Jetpack Surfaces Row Handle`))
  (`LPSPExplosionComponent.StartShake` (`self.Jetpack Explosion`) 0)
  (`LPSPExplosionComponent.TryApplyDamage` :`self` (`self.Jetpack Explosion`))
  (`|ExecutionSequence`
    (:`then_0`
      (`KismetSystemLibrary.Delay` 0.1)
      (`LPSPExplosionComponent.TryApplyImpulse` :`self` (`self.Jetpack Explosion`)))))

(fn `UserConstructionScript`
  (`parent.UserConstructionScript`))